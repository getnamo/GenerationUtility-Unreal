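; UnrealJsRuntime is a Blueprint that supports a JavaScript instance with script change notifications and name-keyed reference lookups.
; On BeginPlay, if enabled in settings, it creates DirectoryWatchers for the project's Content/Scripts folder and the Generation-Utility-Unreal plugin's scripts folder.
; On each change, it emits only the first modified file to the JavaScript instance as an "onFileChanged" message.
; Helper functions turn the object and class reference lists into maps keyed by name.
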(event `self.ReceiveBeginPlay`
  (if (`.WatchDirectoriesForChange_1_C3487E8A44ED45FAC3B5D3A0D82A7DAF` (break `/GenerationUtility/Blueprint/JsRuntimeSettings` (`self.Settings`)))
    (`self.WatchDirectories`)))

(event `WatchDirectories`
  (`|ExecutionSequence`
    (:`then_0`
      (bind _returnvalue (`|GenericCreateObject` "/Script/V8.DirectoryWatcher"))
      (bind _output_get (set `self.ProjectFileWatcher` _returnvalue))
      (add `DirectoryWatcher.OnChanged` _output_get (delegate `OnProjectFileChanged`))
      (`DirectoryWatcher.Watch` _output_get (`KismetStringLibrary.Concat_StrStr` (`CUFileSubsystem.ProjectDirectory` (subsystem `CUFileSubsystem`)) "Content/Scripts")))
    (:`then_1`
      (bind _returnvalue_2 (`|GenericCreateObject` "/Script/V8.DirectoryWatcher"))
      (bind _output_get_2 (set `self.GUFileWatcher` _returnvalue_2))
      (add `DirectoryWatcher.OnChanged` _output_get_2 (delegate `OnGUFileChanged`))
      (`DirectoryWatcher.Watch` _output_get_2 (`KismetStringLibrary.Concat_StrStr` (`CUFileSubsystem.ProjectDirectory` (subsystem `CUFileSubsystem`)) "Plugins/OpenSource/Generation-Utility-Unreal/Content/Scripts")))))

(event `OnProjectFileChanged`
  (`self.OnWatchedFileChanged` (`|GetArrayItem` (`DirectoryWatcher.Modified` (`self.ProjectFileWatcher`)))))

(event `OnGUFileChanged`
  (`self.OnWatchedFileChanged` (`|GetArrayItem` (`DirectoryWatcher.Modified` (`self.GUFileWatcher`)))))

(fn `GetClassReferenceMap`
  (returns (cmap :type "Map of String to Object Class Reference"))
  (locals (TempCmap :type "Map of String to Object Class Reference"))
  (for _array_element (`self.ClassReferenceList`)
    (`BlueprintMapLibrary.Map_Add` (`local.TempCmap`) (`KismetSystemLibrary.GetClassDisplayName` _array_element) _array_element))
  (return (`local.TempCmap`)))

(fn `GetObjectReferenceMap`
  (returns (omap :type "Map of String to Object Object Reference"))
  (locals (TempOmap :type "Map of String to Object Object Reference"))
  (for _array_element (`self.ObjectReferenceList`)
    (`BlueprintMapLibrary.Map_Add` (`local.TempOmap`) (`KismetSystemLibrary.GetObjectName` _array_element) _array_element))
  (return (`local.TempOmap`)))

(fn `OnWatchedFileChanged`
  (params (File :type String))
  (`JavascriptInstanceComponent.Emit` (`self.JavascriptInstance`) "onFileChanged" File))

(fn `UserConstructionScript`)